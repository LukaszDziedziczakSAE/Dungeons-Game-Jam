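; Projectile actor for the medieval weapons set that sticks into whatever it hits.
; Its ProjectileMovement component drives flight, and all custom logic runs when that component reports a stop.
; On stop it spawns an impact effect, teleports slightly forward along the mesh to embed itself, and deactivates its particle system.
; It attaches to the hit component at the hit bone, keeping world transform, so it follows moving targets.
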(event OnProjectileStop(ProjectileMovement)
  (params (ImpactResult :type Hit%20Result%20Structure%20%28by%20ref%29))
  (bind (_bblockinghit _binitialoverlap _time _distance _location _impactpoint _normal _impactnormal _physmat _hitactor _hitcomponent _hitbonename) (Collision|BreakHitResult ImpactResult))
  (bind _staticmesh (Variables|Default|GetStaticMesh))
  (Effects|SpawnEmitteratLocation "/Game/Medieval_Weapons/VFX/P_Impact.P_Impact" _location "0, 0, 0" "2.000000,2.000000,2.000000")
  (Transformation|SetActorLocation (+ (Transformation|GetWorldLocation _staticmesh) (* (Math|Vector|GetForwardVector _staticmesh) (Math|Float|MakeLiteralFloat 4e+01))) false true)
  (Transformation|AttachComponentToComponent _hitcomponent _hitbonename "KeepWorld" "KeepWorld" "KeepWorld" true)
  (Components|Activation|Deactivate (Variables|Default|GetParticleSystem)))

(event Collision|EventActorBeginOverlap
  (params (OtherActor :type Actor%20Object%20Reference)))

(event EventTick
  (params (DeltaSeconds :type Float%20%28single-precision%29)))

(fn ConstructionScript)